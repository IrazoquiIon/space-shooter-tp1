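; Player spaceship Blueprint that handles the UI, sound and visual feedback for gameplay events raised outside this graph.
; Lives and score changes are forwarded to WBP_HUD, and game over passes the final score to WBP_GameOver with a lose sound.
; A HUDReady flag skips the shield-down sound on the first lives update.
; Firing plays a laser sound and briefly shows the muzzle flash using a Delay.
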(event EventBeginPlay)

(event Collision|EventActorBeginOverlap
  (params (OtherActor :type Actor%20Object%20Reference)))

(event EventTick
  (params (DeltaSeconds :type Float%20%28single-precision%29)))

(event EventOnLivesChanged
  (params (NewLives :type Integer))
  (bind _aswbp_hud (Utilities|Casting|CastToWBP_HUD (Variables|Default|GetHUDWidgetInstance)))
  (Default|UpdateLives _aswbp_hud NewLives)
  (if (Variables|Default|GetbHUDReady)
    (Audio|PlaySound2D "/Game/Sounds/sfx_shieldDown.sfx_shieldDown" 1.0 1.0 0.0 0 0)
    (else
      (Variables|Default|SetbHUDReady true))))

(event EventOnScoreChanged
  (params (NewScore :type Integer))
  (bind _aswbp_hud (Utilities|Casting|CastToWBP_HUD (Variables|Default|GetHUDWidgetInstance)))
  (Default|UpdateScore _aswbp_hud NewScore))

(event EventOnGameOver
  (params (GameOverWidget :type User%20Widget%20Object%20Reference) (FinalScore :type Integer))
  (bind _aswbp_game_over (Utilities|Casting|CastToWBP_GameOver GameOverWidget))
  (Default|SetFinalScore _aswbp_game_over FinalScore)
  (Audio|PlaySound2D "/Game/Sounds/sfx_lose.sfx_lose" 1.0 1.0 0.0 0 0))

(event EventOnFire
  (Audio|PlaySound2D "/Game/Sounds/sfx_laser1.sfx_laser1" 1.0 1.0 0.0 0 0)
  (Rendering|SetVisibility (Variables|Default|GetMuzzleFlash) true false)
  (Utilities|FlowControl|Delay 0.05)
  (Rendering|SetVisibility (Variables|Default|GetMuzzleFlash) false false))

(fn ConstructionScript)